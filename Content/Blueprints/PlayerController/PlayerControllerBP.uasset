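; Player control Blueprint with a mouse cursor and WASD camera for selecting and moving characters, apparently turn-based.
; A Tick-driven six-state machine runs exit, enter and update handlers when NextState changes, though most are stubs or prints.
; Cursor traces select clickable characters, deselect on floor clicks, and spawn characters with Q.
; Character Selected adds an Enhanced Input action context, where key 1 moves the character to the cursor.
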(event EventBeginPlay
  (|SetInputcontext)
  (|ShowMouse)
  (Variables|Default|SetCurrentState "NewEnumerator0"))

(event Collision|EventActorBeginOverlap
  (params (OtherActor :type Actor%20Object%20Reference)))

(event EventTick
  (params (DeltaSeconds :type Float%20%28single-precision%29))
  (CallFunction|StateMachineUpdate))

(event Custom|StateMachineUpdate
  (if (!= (Math|Conversions|ToInteger(Byte) (Variables|Default|GetCurrentState)) (Math|Conversions|ToInteger(Byte) (Variables|Default|GetNextState)))
    (switch Utilities|FlowControl|Switch|SwitchonPlayerStates (Variables|Default|GetCurrentState)
      (:NewEnumerator0
        ;[1 1 1] OnExits
        (|ReadyStateExit))
      (:NewEnumerator1
        (|IdleStateExit))
      (:NewEnumerator2
        (|CharacterSelectedExit))
      (:NewEnumerator3
        (|SelectingTargetExit))
      (:NewEnumerator4
        (|PerformingActionExit))
      (:NewEnumerator5
        (|NotMyStateExit)))
    (bind _output_get (Variables|Default|SetCurrentState (Variables|Default|GetNextState)))
    (switch Utilities|FlowControl|Switch|SwitchonPlayerStates _output_get
      (:NewEnumerator0
        ;[1 1 1] OnEnters
        (|ReadyStateEnter))
      (:NewEnumerator1
        (|IdleStateEnter))
      (:NewEnumerator2
        (|CharacterSelectedStateEnter))
      (:NewEnumerator3
        (|SelectingTargetStateEnter))
      (:NewEnumerator4
        (|PerformingActionStateEnter))
      (:NewEnumerator5
        (|NotMyTurnStateEnter))))
  (switch Utilities|FlowControl|Switch|SwitchonPlayerStates (Variables|Default|GetCurrentState)
    (:NewEnumerator0
      ;[1 1 1] StateUpdates
      (|ReadyStateLogic))
    (:NewEnumerator1
      (|IdleStateLogic))
    (:NewEnumerator2
      (|CharacterSelectedStateLogic))
    (:NewEnumerator3
      (|SelectingTargetStateLogic))
    (:NewEnumerator4
      (|PerformingActionStateLogic))
    (:NewEnumerator5
      (|NotMyTurnStateLogic))))

(event Custom|ChangeState
  (params (state :type PlayerStates%20Enum :default "NewEnumerator0"))
  ;[1 1 1] Comment
  (Variables|Default|SetNextState state))

(fn ConstructionScript)

(fn SelectTarget
  (params (Target :type My%20Character%20Object%20Reference))
  ;[1 1 1] Deselect old taget if valid
  (Utilities|IsValid (Variables|Default|GetSelectedCharacter)
    (:Is%20Valid
      (bind _output_get (LocalVariables|SetOldTargetStored (Variables|Default|GetSelectedCharacter)))
      (Default|GetDeselected _output_get))
    (:Is%20Not%20Valid
      _))
  (bind _output_get_2 (Variables|Default|SetSelectedCharacter Target))
  (Default|GetSelected _output_get_2)
  (CallFunction|ChangeState "NewEnumerator2"))

(event Input|EnhancedActionEvents|EnhancedInputActionAction_Camera_Movement
  (params (ActionValue :type Vector%202D%20Structure) (ElapsedSeconds :type Float%20%28double-precision%29) (TriggeredSeconds :type Float%20%28double-precision%29) (InputAction :type Input%20Action%20Object%20Reference :default "/Game/Input/Actions/Camera_Actions/Action_Camera_Movement.Action_Camera_Movement"))
  (bind (_returnvalue _returnvalue2) (|PickCameraVectors))
  (bind _defaultsceneroot (Variables|Default|GetDefaultSceneRoot))
  (bind _movespeed (Variables|Default|GetMoveSpeed))
  (:Triggered
    (Transformation|AddLocalOffset _defaultsceneroot (* (.x ActionValue) (* _returnvalue _movespeed)) false false)
    (Transformation|AddLocalOffset _defaultsceneroot (* (* _movespeed _returnvalue2) (.y ActionValue)) false false)
    (return)))

(event Input|EnhancedActionEvents|EnhancedInputActionAction_Q
  (params (ActionValue :type Boolean) (ElapsedSeconds :type Float%20%28double-precision%29) (TriggeredSeconds :type Float%20%28double-precision%29) (InputAction :type Input%20Action%20Object%20Reference :default "/Game/Input/Actions/Camera_Actions/Action_Q.Action_Q"))
  (bind _camera (Variables|Default|GetCamera))
  (bind _returnvalue (Transformation|GetWorldLocation _camera))
  (:Started
    (bind _outhit (Collision|LineTraceByChannel _returnvalue (+ _returnvalue (* (.WorldDirection (Game|Player|ConvertMouseLocationToWorldSpace (Game|GetPlayerController 0))) 9999.0)) "TraceTypeQuery1" false 0 "None"))
    (Game|SpawnActorfromClass "/Game/Blueprints/Characters/AlliedCharacters/MainCharacter.MainCharacter_C" (Math|Transform|MakeTransform (+ (.location _outhit) "0.000000,0.000000,100.000000") "0, 0, 0" "1.000000,1.000000,1.000000") "Undefined" "MultiplyWithRoot" 0 0)
    (return)))

(event Input|EnhancedActionEvents|EnhancedInputActionAction_Click
  (params (ActionValue :type Boolean) (ElapsedSeconds :type Float%20%28double-precision%29) (TriggeredSeconds :type Float%20%28double-precision%29) (InputAction :type Input%20Action%20Object%20Reference :default "/Game/Input/Actions/Camera_Actions/Action_Click.Action_Click"))
  (bind (_returnvalue _returnvalue2) (|PickCameraStartAndDirection))
  (:Started
    (bind _outhit (Collision|LineTraceByChannel _returnvalue _returnvalue2 "TraceTypeQuery1" false 0 "None"))
    ;[1 1 1] Clickable?
    (if (Utilities|DoesObjectImplementInterface (.hitactor _outhit) "/Game/Blueprints/Characters/Interfaces/ClickableInterface.ClickableInterface_C")
      ;[1 1 1] Check if we are on a state that can select characters
      (|CheckState
        (:then
          (Class|ClickableInterface|GetClicked(Message) (.hitactor _outhit))
          (bind _asmy_character (Utilities|Casting|CastToMyCharacter (.hitactor _outhit)))
          (CallFunction|SelectTarget _asmy_character))
        (:else
          _))
      (else
        (|FloorClick
          (:else
            _)
          (:then
            _))))
    (return)))

(event Input|EnhancedActionEvents|EnhancedInputActionAction_2
  (params (ActionValue :type Boolean) (ElapsedSeconds :type Float%20%28double-precision%29) (TriggeredSeconds :type Float%20%28double-precision%29) (InputAction :type Input%20Action%20Object%20Reference :default "/Game/Input/Actions/CharacterActions/Action_2.Action_2"))
  (:Started
    (Development|PrintString "Key 2 pressed")))

(event Input|EnhancedActionEvents|EnhancedInputActionAction_1
  (params (ActionValue :type Boolean) (ElapsedSeconds :type Float%20%28double-precision%29) (TriggeredSeconds :type Float%20%28double-precision%29) (InputAction :type Input%20Action%20Object%20Reference :default "/Game/Input/Actions/CharacterActions/Action_1.Action_1"))
  (bind (_returnvalue _returnvalue2) (|PickCameraStartAndDirection_2))
  (bind _selectedcharacter (Variables|Default|GetSelectedCharacter))
  (bind _defaultsceneroot (Variables|/Game/Blueprints/Characters/MyCharacter.MyCharacter_C|GetDefaultSceneRoot _selectedcharacter))
  (:Triggered
    (bind _outhit (Collision|LineTraceByChannel _returnvalue _returnvalue2 "TraceTypeQuery1" false 0 "None"))
    (Transformation|SetWorldLocation _defaultsceneroot (Math|Vector|MakeVector (.x (Math|Vector2D|MakeVector2D (.x (.location _outhit)) (.y (.location _outhit)))) (.y (Math|Vector2D|MakeVector2D (.x (.location _outhit)) (.y (.location _outhit)))) (.z (Transformation|GetWorldLocation _defaultsceneroot))) false false)))

(event Input|EnhancedActionEvents|EnhancedInputActionAction_Click
  (params (ActionValue :type Boolean) (ElapsedSeconds :type Float%20%28double-precision%29) (TriggeredSeconds :type Float%20%28double-precision%29) (InputAction :type Input%20Action%20Object%20Reference :default "/Game/Input/Actions/Camera_Actions/Action_Click.Action_Click")))
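; DummdefaultPawn is a camera pawn that moves on input and spawns DummySpawnable actors on click.
; BeginPlay adds the Camera_Context Enhanced Input mapping.
; Movement input offsets the root locally along the camera's forward and right vectors, flattened to XY and scaled by MoveSpeed.
; Clicking traces the Visibility channel from the camera's forward view and spawns above the hit location, without checking for a hit.
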(event Input|EnhancedActionEvents|EnhancedInputActionAction_Click
  (params (ActionValue :type Boolean) (ElapsedSeconds :type Float%20%28double-precision%29) (TriggeredSeconds :type Float%20%28double-precision%29) (InputAction :type Input%20Action%20Object%20Reference :default "/Game/Input/Actions/Camera_Actions/Action_Click.Action_Click"))
  (bind _camera (Variables|Default|GetCamera))
  (:Started
    (bind _outhit (Collision|LineTraceByChannel (Transformation|GetWorldLocation (Variables|Default|GetCamera)) (+ (Transformation|GetWorldLocation _camera) (* (Math|Vector|GetForwardVector _camera) 999999.0)) "TraceTypeQuery1" false 0 "None"))
    (Game|SpawnActorfromClass "/Game/Blueprints/Spawnables/DummySpawnable.DummySpawnable_C" (Math|Transform|MakeTransform (+ (.location _outhit) "0.000000,0.000000,100.000000") "0, 0, 0" "1.000000,1.000000,1.000000") "Undefined" "MultiplyWithRoot" 0 0)))

(event EventBeginPlay
  (Input|AddMappingContext (PlayerController|LocalPlayerSubsystems|GetEnhancedInputLocalPlayerSubsystem (Game|GetPlayerController 0)) "/Game/Input/Camera_Context.Camera_Context" 0 "(bIgnoreAllPressedKeysUntilRelease=True,bForceImmediately=False)")
  (Development|PrintString "Input Context Set"))

(event Collision|EventActorBeginOverlap
  (params (OtherActor :type Actor%20Object%20Reference)))

(event EventTick
  (params (DeltaSeconds :type Float%20%28single-precision%29)))

(fn ConstructionScript)

(event Input|EnhancedActionEvents|EnhancedInputActionAction_Camera_Movement
  (params (ActionValue :type Vector%202D%20Structure) (ElapsedSeconds :type Float%20%28double-precision%29) (TriggeredSeconds :type Float%20%28double-precision%29) (InputAction :type Input%20Action%20Object%20Reference :default "/Game/Input/Actions/Camera_Actions/Action_Camera_Movement.Action_Camera_Movement"))
  (bind _defaultsceneroot (Variables|Default|GetDefaultSceneRoot))
  (bind _movespeed (Variables|Default|GetMoveSpeed))
  (bind _camera (Variables|Default|GetCamera))
  (bind _returnvalue (Math|Vector|GetForwardVector _camera))
  (bind _returnvalue_2 (Math|Vector|GetRightVector _camera))
  (:Triggered
    (Transformation|AddLocalOffset _defaultsceneroot (* (.x ActionValue) (* (Math|Conversions|ToVector(Vector2D) (Math|Vector2D|MakeVector2D (.x _returnvalue) (.y _returnvalue))) _movespeed)) false false)
    (Transformation|AddLocalOffset _defaultsceneroot (* (* _movespeed (Math|Conversions|ToVector(Vector2D) (Math|Vector2D|MakeVector2D (.x _returnvalue_2) (.y _returnvalue_2)))) (.y ActionValue)) false false)))
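; GridBP is a pathfinding test Blueprint that moves a FollowPathBP actor along a grid path.
; FindPath spawns the follower and stores a path between hardcoded points from FindFullPath, defined outside this file, but its call in the event graph is unconnected.
; Tick advances an alpha and waypoint index, linearly interpolating the follower between consecutive points and resetting the index at the last one.
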(event EventBeginPlay)

(event Collision|EventActorBeginOverlap
  (params (OtherActor :type Actor%20Object%20Reference)))

(event EventTick
  (params (DeltaSeconds :type Float%20%28single-precision%29))
  (CallFunction|UpdateIdx DeltaSeconds))

(fn ConstructionScript)

(fn FindPath
  (bind _returnvalue (Game|SpawnActorfromClass "/Game/Blueprints/PathdindingTest/FollowPathBP.FollowPathBP_C" (Math|Transform|MakeTransform "0, 0, 0" "0, 0, 0" "1.000000,1.000000,1.000000") "Undefined" "MultiplyWithRoot" 0 0))
  (Variables|Default|SetFollowPath _returnvalue)
  (Class|GridManager|SetCellSize 150)
  (bind _returnvalue_2 (Class|GridManager|FindFullPath "0, 0, 0" "1500.000000,1500.000000,0.000000"))
  (Variables|Default|SetPath _returnvalue_2))

(fn MoveThroughPath
  (bind _path (Variables|Default|GetPath))
  (bind _newparam1 (CallFunction|IsValidIdx (Variables|Default|GetPathIdx)))
  (if _newparam1
    (bind _newparam1_2 (CallFunction|IsValidIdx (+ (Variables|Default|GetPathIdx) 1)))
    (if _newparam1_2
      (Transformation|SetWorldLocation (Variables|/Game/Blueprints/PathdindingTest/FollowPathBP.FollowPathBP_C|GetDefaultSceneRoot (Variables|Default|GetFollowPath)) (Math|Interpolation|Ease "Linear" (Variables|Default|Gett) (Utilities|Array|Get(acopy) _path (Variables|Default|GetPathIdx)) (Utilities|Array|Get(acopy) _path (+ (Variables|Default|GetPathIdx) 1))) false false)
      (else
        (Variables|Default|SetPathIdx 0)))))

(fn IsValidIdx
  (params (NewParam :type Integer))
  (return (< NewParam (Utilities|Array|Length (Variables|Default|GetPath)))))

(fn UpdateIdx
  (params (A :type Float%20%28double-precision%29))
  (bind _output_get (Variables|Default|Sett (+ (* A (Variables|Default|GetMoveVelocity)) (Variables|Default|Gett))))
  (if (>= _output_get 1.0)
    (Variables|Default|Sett 0.0)
    (Math|Integer|IncrementInt (Variables|Default|GetPathIdx)
      (:%20%20
        _)))
  (CallFunction|MoveThroughPath))
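; Default game mode Blueprint that owns the game's ReferenceManager and can spawn the main character and three minions.
; BeginPlay spawns the ReferenceManager actor at the origin and stores it, with GMGetRefMgr exposing it to callers.
; SpawnCharacters places the main character near the origin with the minions at fixed offsets around it and stores each reference.
; Nothing in this graph calls SpawnCharacters.
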(event EventBeginPlay
  (CallFunction|CreateRefManager))

(event EventTick
  (params (DeltaSeconds :type Float%20%28single-precision%29)))

(fn ConstructionScript)

(fn CreateRefManager
  (bind _returnvalue (Game|SpawnActorfromClass "/Game/Blueprints/ReferenceManager/ReferenceManager.ReferenceManager_C" (Math|Conversions|ToTransform(Vector) (Math|Vector|VectorZero)) "Undefined" "MultiplyWithRoot" 0 0))
  (Variables|Default|SetRefManager _returnvalue))

(fn GMGetRefMgr
  (return (Variables|Default|GetRefManager)))

(fn SpawnCharacters
  (bind _returnvalue (Math|Vector|MakeVector 0.0 0.0 1e+01))
  (bind _returnvalue_2 (+ _returnvalue "400.000000,0.000000,0.000000"))
  (bind _returnvalue_3 (+ _returnvalue "0.000000,400.000000,0.000000"))
  (bind _returnvalue_4 (Game|SpawnActorfromClass "/Game/Blueprints/Characters/AlliedCharacters/MainCharacter.MainCharacter_C" (Math|Conversions|ToTransform(Vector) _returnvalue) "Undefined" "MultiplyWithRoot" 0 0))
  (Variables|Default|SetMainCharacter _returnvalue_4)
  (bind _returnvalue_5 (Game|SpawnActorfromClass "/Game/Blueprints/Characters/AlliedCharacters/Minion1.Minion1_C" (Math|Conversions|ToTransform(Vector) _returnvalue_2) "Undefined" "MultiplyWithRoot" 0 0))
  (Variables|Default|SetMinion1 _returnvalue_5)
  (bind _returnvalue_6 (Game|SpawnActorfromClass "/Game/Blueprints/Characters/AlliedCharacters/Minion2.Minion2_C" (Math|Conversions|ToTransform(Vector) _returnvalue_3) "Undefined" "MultiplyWithRoot" 0 0))
  (Variables|Default|SetMinion2 _returnvalue_6)
  (bind _returnvalue_7 (Game|SpawnActorfromClass "/Game/Blueprints/Characters/AlliedCharacters/Minion3.Minion3_C" (Math|Conversions|ToTransform(Vector) (+ _returnvalue_2 _returnvalue_3)) "Undefined" "MultiplyWithRoot" 0 0))
  ;[1 1 1] Comment
  (Variables|Default|SetMinion3 _returnvalue_7))
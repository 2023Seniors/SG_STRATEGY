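; Grid manager actor that sets up the map's grid dimensions and cell size and provides a toggleable debug view of it.
; On BeginPlay it sets those values, hides its Plane and pre-spawns a hidden GridDebugCellSpawnable at each cell center, offset from the actor's location.
; GridDebugMode flips a flag and shows or hides the stored DebugGrid actors rather than respawning them.
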(event EventBeginPlay
  (Variables|Default|SetDebugMode false)
  (Class|GridManager|SetMapSize 10 10)
  (Class|GridManager|SetCellSize 300)
  (CallFunction|CreateGridDebugArray)
  (Rendering|SetVisibility (Variables|Default|GetPlane) false false))

(event Collision|EventActorBeginOverlap
  (params (OtherActor :type Actor%20Object%20Reference)))

(event EventTick
  (params (DeltaSeconds :type Float%20%28single-precision%29)))

(fn ConstructionScript)

(fn GridDebugMode
  (bind _output_get (Variables|Default|SetDebugMode (not (Variables|Default|GetDebugMode))))
  (if _output_get
    (CallFunction|DisplayGridDebugMode)
    (else
      (CallFunction|HideGridDebugMode))))

(fn CreateGridDebugArray
  (bind _returnvalue (Class|GridManager|GetMapSize))
  (LocalVariables|SetGridSize _returnvalue)
  (bind _returnvalue_2 (Class|GridManager|GetCellSize))
  (LocalVariables|SetCellSize _returnvalue_2)
  (for _index (range 0 (- (Math|Float|Truncate (.x (LocalVariables|GetGridSize))) 1))
    (for _index_2 (range 0 (- (Math|Float|Truncate (.y (LocalVariables|GetGridSize))) 1))
      (bind _output_get (LocalVariables|SetNewLocalVar (+ (+ (.location (Transformation|GetActorTransform)) (Math|Vector|MakeVector (* (LocalVariables|GetCellSize) _index 1.0) (* (LocalVariables|GetCellSize) _index_2 1.0) 0.0)) (/ (LocalVariables|GetCellSize) 2))))
      (bind _returnvalue_3 (Game|SpawnActorfromClass "/Game/Blueprints/Spawnables/GridDebugCellSpawnable.GridDebugCellSpawnable_C" (Math|Transform|MakeTransform (Math|Vector|MakeVector (.x _output_get) (.y _output_get) 0.0) "0, 0, 0" "2.500000,2.500000,1.000000") "Undefined" "MultiplyWithRoot" 0 0))
      (Utilities|Array|Add (Variables|Default|GetDebugGrid) _returnvalue_3)
      (Rendering|SetActorHiddenInGame _returnvalue_3 true)))
  (return))

(fn DisplayGridDebugMode
  (for _array_element (Variables|Default|GetDebugGrid)
    (Rendering|SetActorHiddenInGame _array_element false))
  (return))

(fn HideGridDebugMode
  (for _array_element (Variables|Default|GetDebugGrid)
    (Rendering|SetActorHiddenInGame _array_element true))
  (return))
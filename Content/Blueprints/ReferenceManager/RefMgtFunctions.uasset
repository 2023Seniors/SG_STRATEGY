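; RefMgtFunctions is a set of global accessor functions for the game's manager objects.
; GetRefMgr casts the current game mode to DefaultGamemodeBP and returns the reference manager it holds.
; GetTurnMgr, GetImporter and GetGridMgr each go through GetRefMgr to return the turn manager, importer or grid manager, keeping the reference manager as the single lookup point.
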(fn GetRefMgr
  (bind _asdefault_gamemode_bp (Utilities|Casting|CastToDefaultGamemodeBP (Game|GetGameMode)))
  (bind _refmgr (Default|GMGetRefMgr _asdefault_gamemode_bp))
  (return _refmgr))

(fn GetTurnMgr
  (bind _refmgr (CallFunction|GetRefMgr))
  (bind _turn_mg (Default|GetTurnMgr _refmgr))
  (return _turn_mg))

(fn GetImporter
  (bind _refmgr (CallFunction|GetRefMgr))
  (bind _importer (CallFunction|GetImporter _refmgr))
  (return _importer))

(fn GetGridMgr
  (bind _refmgr (CallFunction|GetRefMgr))
  (bind _grid (Default|GetGridManager _refmgr))
  (return _grid))
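; ReferenceManager is an actor that creates the game's core managers and serves as a central access point for them.
; On BeginPlay it spawns the TurnManager, ImporterBP and GridManagerBP, and adds the HUD widget to the viewport.
; It stores the turn manager, HUD and grid manager directly, while the importer and player controller are assigned through ImImporter and ImPlayerController.
; Getter functions expose each stored reference.
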(event EventBeginPlay
  (|CreateTurnManager)
  (CallFunction|CreateHUD)
  (|CreateImporter)
  (bind _returnvalue (Game|SpawnActorfromClass "/Game/Blueprints/GridManager/GridManagerBP.GridManagerBP_C" (Math|Transform|MakeTransform "0, 0, 0" "0, 0, 0" "1.000000,1.000000,1.000000") "Undefined" "MultiplyWithRoot" 0 0))
  (Variables|Default|SetGridManager _returnvalue))

(event Collision|EventActorBeginOverlap
  (params (OtherActor :type Actor%20Object%20Reference)))

(event EventTick
  (params (DeltaSeconds :type Float%20%28single-precision%29)))

(fn ConstructionScript)

(fn GetTurnMgr
  (return (Variables|Default|GetTurnManager)))

(fn GetHUD
  (return (Variables|Default|GetHUD)))

(fn GetPlayerController
  (return (Variables|Default|GetPlayerController)))

(fn CreateHUD
  (bind _returnvalue (UserInterface|CreateWidget "/Game/Blueprints/ReferenceManager/HUD/HUDWIdget.HUDWIdget_C"))
  (Variables|Default|SetHUD _returnvalue)
  (UserInterface|Viewport|AddtoViewport _returnvalue 0))

(fn ImPlayerController
  (params (pc :type Player%20Controller%20BP%20Object%20Reference))
  (Variables|Default|SetPlayerController pc))

(fn ImImporter
  (params (importer :type Importer%20BP%20Object%20Reference))
  (Variables|Default|SetImporter importer))

(fn GetImporter
  (return (Variables|Default|GetImporter)))

(fn GetGridManager
  (return (Variables|Default|GetGridManager)))